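; Player character Blueprint that equips a sword through a weapon combat component and routes damage and stamina use to a health component.
; Left mouse calls SS, Space spends stamina, and health, stamina and death are shown as debug prints.
; An S_S event toggles movement off and on, stopping the sword attack when walking resumes.
; Disconnected prototype logic picks Left, Right or Top from mouse position for directional attack and block animations.
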(event OnHealthEnded(HealthComponent)
  (CallFunction|PrintMessage 0 "" "Dead" "(R=1.000000,G=0.092311,B=0.000000,A=1.000000)" 3.0))

(event Custom|S_S
  (bind _charactermovement (Variables|Character|GetCharacterMovement))
  (if (not (Variables|Default|GetNewVar_1))
    (Variables|Default|SetNewVar_1 true)
    (Pawn|Components|CharacterMovement|SetMovementMode _charactermovement "MOVE_None" 0)
    (else
      (Variables|Default|SetNewVar_1 false)
      (Pawn|Components|CharacterMovement|SetMovementMode _charactermovement "MOVE_Walking" 0)
      (Class|WeaponCombatComponent|StopSwordAttack (Variables|Default|GetBP_WeaponCombatComponent)))))

(event Custom|TestTrace
  (params (LineStart :type Vector) (LineEnd :type Vector) (LineColor :type Linear%20Color%20Structure) (Duration :type Float%20%28single-precision%29) (Thickness :type Float%20%28single-precision%29))
  (Rendering|Debug|DrawDebugLine LineStart LineEnd LineColor Duration Thickness))

(event EventBeginPlay
  (Class|WeaponCombatComponent|CreateWeaponSword (Variables|Default|GetBP_WeaponCombatComponent) "/Game/Blueprints/Weapons/BP_BaseWeaponSword.BP_BaseWeaponSword_C"))

(event Game|Damage|EventAnyDamage
  (params (Damage :type Float%20%28single-precision%29) (DamageType :type Damage%20Type%20Object%20Reference) (InstigatedBy :type Controller%20Object%20Reference) (DamageCauser :type Actor%20Object%20Reference))
  (Class|HealthComponent|GetDamage (Variables|Default|GetHealthComponent) Damage))

(event EventTick
  (params (DeltaSeconds :type Float%20%28single-precision%29))
  (bind _self self)
  (Utilities|FlowControl|Sequence
    (:then_0
      (CallFunction|PrintMessage _self "Health" (Utilities|String|ToString(Float) (Variables|/Script/KnightCombat.HealthComponent|GetCurrentHealth (Variables|Default|GetHealthComponent))) "(R=1.000000,G=0.000000,B=0.123326,A=1.000000)" 0.0))
    (:then_1
      (CallFunction|PrintMessage _self "Stamina" (Utilities|String|ToString(Float) (Variables|/Script/KnightCombat.HealthComponent|GetCurrentStamina (Variables|Default|GetHealthComponent))) "(R=1.000000,G=0.854708,B=0.000000,A=1.000000)" 0.0))))

(event Input|MouseEvents|LeftMouseButton
  (params (Key :type Key%20Structure :default "None"))
  (:Pressed
    (CallFunction|SS)))

(event Input|MouseEvents|RightMouseButton
  (params (Key :type Key%20Structure :default "None")))

(event Input|KeyboardEvents|SpaceBar
  (params (Key :type Key%20Structure :default "None"))
  (:Pressed
    (Class|HealthComponent|UseStaminaValue (Variables|Default|GetHealthComponent) 13.0)))

(fn ConstructionScript)