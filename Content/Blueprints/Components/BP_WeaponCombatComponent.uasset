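; Weapon combat component that samples the current sword's sweep during an attack, currently only drawing debug arrows, with no hit detection.
; StartTrace stores points interpolated between two weapon mesh sockets and starts a looping timer on Server_TraceAttack.
; Each tick of that timer links current blade points to their previous positions with arrows, then updates the stored points.
; StopTrace clears the timer and the points.
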(event Custom|Server_TraceAttack
  (CallFunction|CustomEvent1))

(event Custom|StartTrace
  (for _index (range 0 (Variables|Default|GetTraceValue))
    (Utilities|Array|Add (Variables|Default|GetBiba) (Math|Vector|Lerp(Vector) (Transformation|GetSocketLocation (Variables|/Script/KnightCombat.BaseWeaponSword|GetWeaponMesh (Class|WeaponCombatComponent|GetCurrentWeaponSword)) (Variables|Default|GetSocketStartName)) (Transformation|GetSocketLocation (Variables|/Script/KnightCombat.BaseWeaponSword|GetWeaponMesh (Class|WeaponCombatComponent|GetCurrentWeaponSword)) (Variables|Default|GetSocketEndName)) (/ (Math|Conversions|ToFloat(Integer) _index) (Variables|Default|GetTraceValue))))
    (bind _returnvalue (Utilities|Time|SetTimerbyFunctionName 0 "Server_TraceAttack" (Variables|Default|GetSwordTracingRate) true))
    (Variables|Default|SetNewVar_0 _returnvalue)))

(event Custom|StopTrace
  (Utilities|Time|ClearandInvalidateTimerbyHandle (Variables|Default|GetNewVar_0))
  (Utilities|Array|Clear (Variables|Default|GetBiba)))

(event Custom|CustomEvent_0
  (params (LineStart :type Vector) (LineEnd :type Vector) (ArrowSize :type Float%20%28single-precision%29) (LineColor :type Linear%20Color%20Structure) (Duration :type Float%20%28single-precision%29) (Thickness :type Float%20%28single-precision%29))
  (Rendering|Debug|DrawDebugArrow LineStart LineEnd ArrowSize LineColor Duration Thickness))

(event Custom|CustomEvent_1
  (if (> (Utilities|Array|Length (Variables|Default|GetBiba)) 0)
    (for _index (range 0 (Variables|Default|GetTraceValue))
      (CallFunction|CustomEvent0 (Math|Vector|Lerp(Vector) (Transformation|GetSocketLocation (Variables|/Script/KnightCombat.BaseWeaponSword|GetWeaponMesh (Class|WeaponCombatComponent|GetCurrentWeaponSword)) (Variables|Default|GetSocketStartName)) (Transformation|GetSocketLocation (Variables|/Script/KnightCombat.BaseWeaponSword|GetWeaponMesh (Class|WeaponCombatComponent|GetCurrentWeaponSword)) (Variables|Default|GetSocketEndName)) (/ (Math|Conversions|ToFloat(Integer) _index) (Variables|Default|GetTraceValue))) (Utilities|Array|Get(acopy) (Variables|Default|GetBiba) _index) 3.0 "(R=1.000000,G=0.000000,B=0.410392,A=1.000000)" 5.0 0.0)
      (Utilities|Array|SetArrayElem (Variables|Default|GetBiba) _index (Math|Vector|Lerp(Vector) (Transformation|GetSocketLocation (Variables|/Script/KnightCombat.BaseWeaponSword|GetWeaponMesh (Class|WeaponCombatComponent|GetCurrentWeaponSword)) (Variables|Default|GetSocketStartName)) (Transformation|GetSocketLocation (Variables|/Script/KnightCombat.BaseWeaponSword|GetWeaponMesh (Class|WeaponCombatComponent|GetCurrentWeaponSword)) (Variables|Default|GetSocketEndName)) (/ (Math|Conversions|ToFloat(Integer) _index) (Variables|Default|GetTraceValue)))))))