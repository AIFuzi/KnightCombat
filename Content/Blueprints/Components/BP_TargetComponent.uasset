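; Player lock-on component for BP_Player that toggles aiming the camera at a nearby pawn.
; Server_Trace runs TargetTrace, which sphere-traces around the player, collects hit pawns, disables orient-to-movement and starts a looping Client_Ta timer.
; Each tick of that timer points control rotation from the spring arm at the first stored target.
; Triggering again restores movement orientation, clears targets and stops the timer; multicast events draw debug shapes.
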(event Custom|Server_Trace
  (CallFunction|TargetTrace))

(event Custom|Multicast_DrawSphere
  (params (Center :type Vector) (Radius :type Float%20%28single-precision%29) (Segments :type Integer) (LineColor :type Linear%20Color%20Structure) (Duration :type Float%20%28single-precision%29) (Thickness :type Float%20%28single-precision%29))
  (Rendering|Debug|DrawDebugSphere Center Radius Segments LineColor Duration Thickness))

(event Custom|Multicast_DrawBox
  (params (Center :type Vector) (Extent :type Vector) (LineColor :type Linear%20Color%20Structure) (Duration :type Float%20%28single-precision%29) (Thickness :type Float%20%28single-precision%29))
  (Rendering|Debug|DrawDebugBox Center Extent LineColor "0, 0, 0" Duration Thickness))

(event Custom|Client_Ta
  (CallFunction|Targeting))

(event Custom|SS
  (params (Orient%20Rotation%20to%20Movement :type Boolean))
  (Variables|/Script/Engine.CharacterMovementComponent|SetbOrientRotationToMovement (Variables|/Script/Engine.Character|GetCharacterMovement (Variables|Default|GetPlayerOwner)) Orient%20Rotation%20to%20Movement)
  (Variables|Default|SetIsTargetActivate (not Orient%20Rotation%20to%20Movement)))

(event EventBeginPlay
  (bind _asbp_player (Utilities|Casting|CastToBP_Player (Components|GetOwner)))
  (Variables|Default|SetPlayerOwner _asbp_player))

(fn TargetTrace
  (bind _playerowner (Variables|Default|GetPlayerOwner))
  (bind _returnvalue (Transformation|GetActorLocation _playerowner))
  (if (not (Variables|Default|GetIsTargetActivate))
    (LocalVariables|SetL_Radius 3.5e+02)
    (CallFunction|MulticastDrawSphere (Transformation|GetActorLocation (Variables|Default|GetPlayerOwner)) (LocalVariables|GetL_Radius) 12 "(R=1.000000,G=0.000000,B=0.266638,A=1.000000)" 3.0 0.0)
    (bind (_outhits _returnvalue_2) (Collision|MultiSphereTraceForObjects _returnvalue _returnvalue (LocalVariables|GetL_Radius) (Utilities|Array|MakeArray "ObjectTypeQuery3") false (Utilities|Array|MakeArray _playerowner) "None"))
    (if _returnvalue_2
      (for _array_element _outhits
        (Utilities|Array|AddUnique (Variables|Default|GetTargetEnemys) (.HitActor (Collision|BreakHitResult _array_element)))
        (CallFunction|MulticastDrawBox (Transformation|GetActorLocation (.HitActor (Collision|BreakHitResult _array_element))) "10.000000,10.000000,10.000000" "(R=0.000000,G=1.000000,B=0.109550,A=1.000000)" 3.0 0.0)
        (CallFunction|SS false)
        (bind _returnvalue_3 (Utilities|Time|SetTimerbyFunctionName 0 "Client_Ta" 0.01 true))
        (Variables|Default|SetTargetTimer _returnvalue_3)))
    (else
      (CallFunction|SS true)
      (Utilities|Array|Clear (Variables|Default|GetTargetEnemys))
      (Utilities|Time|ClearandInvalidateTimerbyHandle (Variables|Default|GetTargetTimer)))))

(fn Targeting
  (bind _output_get (LocalVariables|SetL_CurrentTargeting (Utilities|Array|Get(acopy) (Variables|Default|GetTargetEnemys))))
  (Utilities|IsValid _output_get
    (:Is%20Valid
      (Pawn|SetControlRotation (Pawn|GetController (Variables|Default|GetPlayerOwner)) (Math|Rotator|FindLookatRotation (Transformation|GetWorldLocation (Variables|/Script/KnightCombat.PlayerCharacter|GetSpringArmComponent (Variables|Default|GetPlayerOwner))) (Transformation|GetActorLocation (LocalVariables|GetL_CurrentTargeting)))))
    (:Is%20Not%20Valid
      (CallFunction|PrintMessage 0 "" "ERR" "(R=1.000000,G=0.000000,B=0.103951,A=1.000000)" 5.0))))